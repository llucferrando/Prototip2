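; Policeman NPC that patrols and arrests the player at night.
; When the player character overlaps its ArrestRange outside daytime, as reported by the GameManager, it moves that character back to its initial position.
; It exposes its patrol route through a getter and maps a speed state from idle to sprint onto the movement component's max walk speed.
; DefineState is an empty stub.
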(event OnComponentBeginOverlap(ArrestRange)
  (params (OverlappedComponent :type Primitive%20Component%20Object%20Reference) (OtherActor :type Actor%20Object%20Reference) (OtherComp :type Primitive%20Component%20Object%20Reference) (OtherBodyIndex :type Integer) (bFromSweep :type Boolean) (SweepResult :type Hit%20Result%20Structure%20%28by%20ref%29))
  (bind _asbp_third_person_character (Utilities|Casting|CastToBP_ThirdPersonCharacter OtherActor))
  (bind _returnvalue (Actor|GetActorOfClass "/Game/ThirdPerson/Blueprints/GameLoop/GameManager.GameManager_C"))
  (if (not (Variables|/Game/ThirdPerson/Blueprints/GameLoop/GameManager.GameManager_C|GetisDayTime _returnvalue))
    (Transformation|SetActorLocation _asbp_third_person_character (Variables|/Game/ThirdPerson/Blueprints/BP_ThirdPersonCharacter.BP_ThirdPersonCharacter_C|GetinitPos _asbp_third_person_character) false false)))

(event Custom|DefineState)

(fn ConstructionScript)

(fn GetPatrolRoute
  (return (Variables|AI|GetPatrolRoute)))

(fn SetSpeedPolice
  (params (Speed :type E_SpeedPolicePatrol%20Enum :default "NewEnumerator0"))
  (bind _output_get (Variables|/Script/Engine.CharacterMovementComponent|SetMaxWalkSpeed (Variables|Character|GetCharacterMovement) (Utilities|Select :Index Speed :NewEnumerator0 0.0 :NewEnumerator1 3e+02 :NewEnumerator2 4e+02 :NewEnumerator3 6e+02)))
  (return _output_get))